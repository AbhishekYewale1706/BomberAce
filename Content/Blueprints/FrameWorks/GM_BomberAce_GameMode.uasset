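; Game mode for the BomberAce plane game that tracks level progress and the player's Coin and Diamond currencies.
; On BeginPlay it loads saved currency and shows the gameplay HUD widget.
; LevelUpdate advances a progress bar that Tick watches; when full, a one-shot delayed Win pauses the game, awards currency, shows the level-completed screen and saves.
; Save and load share the "Coin" PlaneSaveGame slot, creating it if missing.
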(event `self.ReceiveBeginPlay`
  (`self.LoadData`)
  (bind _returnvalue (`|CreateWidget` "/Game/Blueprints/HUD/WB_GamePlay.WB_GamePlay_C"))
  (bind _output_get (set `self.WB_GameplayRef` _returnvalue))
  (`UserWidget.AddToViewport` _output_get 0))

(event `self.ReceiveTick`
  (params (DeltaSeconds :type "Float (single-precision)"))
  (if (>= (`self.level progress bar`) 1.0)
    (`/Engine/EditorBlueprintResources/StandardMacros.DoOnce` false
      (:`Completed`
        (`KismetSystemLibrary.Delay` 1.0)
        (`GameplayStatics.SetGamePaused` true)
        (`self.Win`)))))

(event `Win`
  (bind _returnvalue (`|CreateWidget` "/Game/Blueprints/HUD/WB_LevelCompleted.WB_LevelCompleted_C"))
  (set `self.AsWB_WinRef` _returnvalue)
  (set `self.Coin` (+ (`self.Coin`) 200))
  (set `self.Diamond` (+ (`self.Diamond`) 20))
  (`UserWidget.AddToViewport` (`self.AsWB_WinRef`) 0)
  (`self.SaveData`))

(event `LevelUpdate`
  (set `self.level progress bar` (+ (`self.level progress bar`) (`self.levelpoint`))))

(event `SaveData`
  (bind _returnvalue (`GameplayStatics.DoesSaveGameExist` "Coin" :!label _label))
  (if _returnvalue
    (bind _returnvalue_2 (`GameplayStatics.LoadGameFromSlot` "Coin"))
    (bind _asplane_save_game (cast `/Game/Blueprints/SaveGame/PlaneSaveGame` _returnvalue_2))
    (`/Engine/EditorBlueprintResources/StandardMacros.IsValid` _asplane_save_game
      (:`Is Valid`
        (set `/Game/Blueprints/SaveGame/PlaneSaveGame.Coin` (`self.Coin`) _asplane_save_game)
        (set `/Game/Blueprints/SaveGame/PlaneSaveGame.Diamond` (`self.Diamond`) _asplane_save_game)
        (`GameplayStatics.SaveGameToSlot` _returnvalue_2 "Coin")))
    (else
      (bind _returnvalue_3 (`GameplayStatics.CreateSaveGameObject` "/Game/Blueprints/SaveGame/PlaneSaveGame.PlaneSaveGame_C"))
      (`GameplayStatics.SaveGameToSlot` _returnvalue_3 "Coin")
      (goto _label))))

(event `LoadData`
  (bind _returnvalue (`GameplayStatics.DoesSaveGameExist` "Coin" :!label _label_2))
  (if _returnvalue
    (bind _returnvalue_2 (`GameplayStatics.LoadGameFromSlot` "Coin"))
    (bind _asplane_save_game (cast `/Game/Blueprints/SaveGame/PlaneSaveGame` _returnvalue_2))
    (`/Engine/EditorBlueprintResources/StandardMacros.IsValid` _asplane_save_game
      (:`Is Valid`
        (set `self.Coin` (`/Game/Blueprints/SaveGame/PlaneSaveGame.Coin` _asplane_save_game))
        (set `self.Diamond` (`/Game/Blueprints/SaveGame/PlaneSaveGame.Diamond` _asplane_save_game))))
    (else
      (bind _returnvalue_3 (`GameplayStatics.CreateSaveGameObject` "/Game/Blueprints/SaveGame/PlaneSaveGame.PlaneSaveGame_C"))
      (`GameplayStatics.SaveGameToSlot` _returnvalue_3 "Coin")
      (goto _label_2))))

(fn `UserConstructionScript`)