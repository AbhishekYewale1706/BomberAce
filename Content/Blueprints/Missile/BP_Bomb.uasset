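; BP_Bomb is an explosive actor that detonates on impact and deals area damage.
; The first hit on its Box component spawns a grenade explosion effect and sound at the impact point, applies radial damage with falloff, then destroys the bomb after a brief delay.
; A DoOnce prevents repeat detonations, and the player pawn is excluded from the damage.
; A bomb that hits nothing destroys itself after a few seconds.
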(event `self.ReceiveBeginPlay`
  (`KismetArrayLibrary.Array_Add` (`self.Ignore Actors`) (`GameplayStatics.GetPlayerPawn` 0))
  (`KismetSystemLibrary.Delay` 5.0)
  (`self.K2_DestroyActor`))

(event `self.Box.OnComponentHit`
  (params (HitComponent :type "PrimitiveComponent Object Reference") (OtherActor :type "Actor Object Reference") (OtherComp :type "PrimitiveComponent Object Reference") (NormalImpulse :type "Vector Structure") (Hit :type "HitResult Structure (by ref)"))
  (bind (_bblockinghit _binitialoverlap _time _distance _location _impactpoint) (`GameplayStatics.BreakHitResult` Hit))
  (`/Engine/EditorBlueprintResources/StandardMacros.DoOnce` false
    (:`Completed`
      (`GameplayStatics.SpawnEmitterAtLocation` "/Game/MilitaryWeapSilver/FX/P_Grenade_Explosion_01.P_Grenade_Explosion_01" _impactpoint (struct) (0.5 0.5 0.5))
      (`GameplayStatics.PlaySoundAtLocation` "/Game/MilitaryWeapSilver/Sound/GrenadeLauncher/Wavs/GrenadeLauncher_Explosion01.GrenadeLauncher_Explosion01" _impactpoint (struct) 1.0 1.0 0.0 null null null null)
      (`self.Apply Radial Damage` _impactpoint)
      (`KismetSystemLibrary.Delay` 0.2)
      (`self.K2_DestroyActor`))))

(event `Apply Radial Damage`
  (params (Origin :type "Vector Structure (by ref)"))
  (`GameplayStatics.ApplyRadialDamageWithFalloff` 50.0 10.0 Origin 100.0 300.0 1.0 null (`self.Ignore Actors`) null null))

(fn `UserConstructionScript`)