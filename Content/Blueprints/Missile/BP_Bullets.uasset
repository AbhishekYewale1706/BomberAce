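; BP_Bullets is a projectile actor that damages player-tagged actors it touches.
; Its Box overlap checks the other actor for the Player tag, applies a small fixed damage, spawns a metal impact effect and hit sound at that actor's location, then destroys itself.
; Overlaps with untagged actors are ignored, and the bullet otherwise destroys itself after a short delay from BeginPlay.
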(event `self.ReceiveBeginPlay`
  (`KismetSystemLibrary.Delay` 5.0)
  (`self.K2_DestroyActor`))

(event `self.Box.OnComponentBeginOverlap`
  (params (OverlappedComponent :type "PrimitiveComponent Object Reference") (OtherActor :type "Actor Object Reference") (OtherComp :type "PrimitiveComponent Object Reference") (OtherBodyIndex :type Integer) (bFromSweep :type Boolean) (SweepResult :type "HitResult Structure (by ref)"))
  (`/Engine/EditorBlueprintResources/StandardMacros.IsValid` OtherActor
    (:`Is Valid`
      (if (`self.ActorHasTag` OtherActor "Player")
        (bind _output_get (set `self.Other Actor(PlayerRef)` OtherActor))
        (`GameplayStatics.ApplyDamage` _output_get 5.0)
        (bind _returnvalue (`self.K2_GetActorLocation` _output_get))
        (`GameplayStatics.SpawnEmitterAtLocation` "/Game/Assets/FX/P_Impact_Metal_Large_01.P_Impact_Metal_Large_01" _returnvalue)
        (`GameplayStatics.PlaySoundAtLocation` "/Game/Assets/Sounds/080884_bullet-hit-39872.080884_bullet-hit-39872" _returnvalue (struct) 1.0 1.0 0.0 null null null null)
        (`self.K2_DestroyActor`)))))

(fn `UserConstructionScript`)