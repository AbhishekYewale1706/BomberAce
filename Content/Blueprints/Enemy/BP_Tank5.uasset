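; BP_Tank5 is an enemy tank that fires at the player and can be destroyed by radial damage.
; The player entering TragetViewerSphere starts looping timers that pitch the mesh toward them (pitch only) and spawn BP_Bullets from the Arrow; leaving clears both.
; Damage updates the WB_EnemyHealth bar; at zero health the tank explodes, calls LevelUpdate on the GameMode and destroys itself.
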(event `self.ReceiveBeginPlay`
  (bind _aswb_enemy_health (cast `/Game/Blueprints/HUD/WB_EnemyHealth` (`WidgetComponent.GetWidget` (`self.Healthbar`))))
  (set `self.As WB Enemy Health` _aswb_enemy_health)
  (bind _asgm_bomber_ace_game_mode (cast `/Game/Blueprints/FrameWorks/GM_BomberAce_GameMode` (`GameplayStatics.GetGameMode`)))
  (set `self.As GM Bomber Ace Game Mode_0` _asgm_bomber_ace_game_mode))

(event `self.ReceiveRadialDamage`
  (params (DamageReceived :type "Float (single-precision)") (DamageType :type "DamageType Object Reference") (Origin :type "Vector Structure") (HitInfo :type "HitResult Structure (by ref)") (InstigatedBy :type "Controller Object Reference") (DamageCauser :type "Actor Object Reference"))
  (bind _returnvalue (`self.K2_GetActorLocation`))
  (bind _output_get (set `self.Health` (- (`self.Health`) DamageReceived)))
  (`ProgressBar.SetPercent` (`/Game/Blueprints/HUD/WB_EnemyHealth.EnemyHealthBar` (`self.As WB Enemy Health`)) (/ _output_get 150.0))
  (if (<= _output_get 0.0)
    (`GameplayStatics.SpawnEmitterAtLocation` "/Game/Assets/FX/P_Grenade_Explosion_01.P_Grenade_Explosion_01" _returnvalue)
    (`GameplayStatics.PlaySoundAtLocation` "/Game/Assets/Sounds/GrenadeLauncher_Explosion01.GrenadeLauncher_Explosion01" _returnvalue (struct) 1.0 1.0 0.0 null null null null)
    (`KismetSystemLibrary.Delay` 0.2)
    (`/Game/Blueprints/FrameWorks/GM_BomberAce_GameMode.LevelUpdate` (`self.As GM Bomber Ace Game Mode_0`))
    (`self.K2_DestroyActor`)))

(event `self.TragetViewerSphere.OnComponentEndOverlap`
  (params (OverlappedComponent :type "PrimitiveComponent Object Reference") (OtherActor :type "Actor Object Reference") (OtherComp :type "PrimitiveComponent Object Reference") (OtherBodyIndex :type Integer))
  (`/Engine/EditorBlueprintResources/StandardMacros.IsValid` OtherActor
    (:`Is Valid`
      (if (`self.ActorHasTag` OtherActor "Player")
        (`self.Other Actor(Player)`
          (:`then`
            (`KismetSystemLibrary.K2_ClearAndInvalidateTimerHandle` (`self.stopshooting`))
            (`KismetSystemLibrary.K2_ClearAndInvalidateTimerHandle` (`self.TimeRef`)))
          (:`else`))))))

(event `self.TragetViewerSphere.OnComponentBeginOverlap`
  (params (OverlappedComponent :type "PrimitiveComponent Object Reference") (OtherActor :type "Actor Object Reference") (OtherComp :type "PrimitiveComponent Object Reference") (OtherBodyIndex :type Integer) (bFromSweep :type Boolean) (SweepResult :type "HitResult Structure (by ref)"))
  (`/Engine/EditorBlueprintResources/StandardMacros.IsValid` OtherActor
    (:`Is Valid`
      (if (`self.ActorHasTag` OtherActor "Player")
        (set `self.Other Actor(Player)` OtherActor)
        (`self.tracktraget`)))))

(event `tracktraget`
  (bind _returnvalue (`KismetSystemLibrary.K2_SetTimerDelegate` (delegate `MoveTurrent`) 0.05 true))
  (set `self.TimeRef` _returnvalue)
  (bind _returnvalue_2 (`KismetSystemLibrary.K2_SetTimerDelegate` (delegate `shooting`) 1.0 true))
  (set `self.stopshooting` _returnvalue_2))

(event `MoveTurrent`
  (bind _other_actor_player_ (`self.Other Actor(Player)`))
  (bind _staticmesh (`self.StaticMesh`))
  (bind (_returnvalue_roll _returnvalue_pitch) (`KismetMathLibrary.BreakRotator` (`KismetMathLibrary.RInterpTo` (`SceneComponent.RelativeRotation` _staticmesh) (`KismetMathLibrary.FindLookAtRotation` (`self.K2_GetActorLocation`) (`self.K2_GetActorLocation` _other_actor_player_)) (`GameplayStatics.GetWorldDeltaSeconds`) 100.0)))
  (`/Engine/EditorBlueprintResources/StandardMacros.IsValid` _other_actor_player_
    (:`Is Valid`
      (`SceneComponent.K2_SetRelativeRotation` _staticmesh (`KismetMathLibrary.MakeRotator` 0.0 _returnvalue_pitch) false false))))

(event `shooting`
  (bind (_returnvalue_location _returnvalue_rotation) (`KismetMathLibrary.BreakTransform` (`SceneComponent.K2_GetComponentToWorld` (`self.Arrow`))))
  (`|SpawnActorFromClass` "/Game/Blueprints/Missile/BP_Bullets.BP_Bullets_C" (`KismetMathLibrary.MakeTransform` _returnvalue_location _returnvalue_rotation) "Undefined" "MultiplyWithRoot" null null)
  (`GameplayStatics.PlaySoundAtLocation` "/Game/Assets/Sounds/RifleA_Fire02.RifleA_Fire02" _returnvalue_location (struct) 1.0 1.0 0.0 null null null null))

(fn `UserConstructionScript`)