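; BP_Tank7 is a destructible enemy tank that takes radial damage and shows its remaining health on a WB_EnemyHealth widget bar.
; A DamageArea overlap tracks whether the Player-tagged plane is in range.
; At zero health it spawns an explosion effect and sound, damages the plane if in range, then after a short delay calls LevelUpdate on GM_BomberAce_GameMode and destroys itself.
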(event `self.ReceiveBeginPlay`
  (bind _aswb_enemy_health (cast `/Game/Blueprints/HUD/WB_EnemyHealth` (`WidgetComponent.GetWidget` (`self.HealthBar`))))
  (set `self.As WB Enemy Health` _aswb_enemy_health)
  (bind _asgm_bomber_ace_game_mode (cast `/Game/Blueprints/FrameWorks/GM_BomberAce_GameMode` (`GameplayStatics.GetGameMode`)))
  (set `self.As GM Bomber Ace Game Mode_0` _asgm_bomber_ace_game_mode))

(event `self.ReceiveTick`
  (params (DeltaSeconds :type "Float (single-precision)")))

(event `self.ReceiveRadialDamage`
  (params (DamageReceived :type "Float (single-precision)") (DamageType :type "DamageType Object Reference") (Origin :type "Vector Structure") (HitInfo :type "HitResult Structure (by ref)") (InstigatedBy :type "Controller Object Reference") (DamageCauser :type "Actor Object Reference"))
  (bind _returnvalue (`self.K2_GetActorLocation`))
  (bind _output_get (set `self.Health` (- (`self.Health`) DamageReceived)))
  (`ProgressBar.SetPercent` (`/Game/Blueprints/HUD/WB_EnemyHealth.EnemyHealthBar` (`self.As WB Enemy Health`)) (/ _output_get 200.0))
  (if (<= _output_get 0.0)
    (`GameplayStatics.SpawnEmitterAtLocation` "/Game/Assets/FX/P_Grenade_Explosion_01.P_Grenade_Explosion_01" _returnvalue)
    (`GameplayStatics.PlaySoundAtLocation` "/Game/Assets/Sounds/GrenadeLauncher_Explosion01.GrenadeLauncher_Explosion01" _returnvalue (struct) 1.0 1.0 0.0 null null null null)
    (if (`self.PlaneInRange`)
      (`GameplayStatics.ApplyDamage` (`self.Other Actor`) 20.0))
    (`KismetSystemLibrary.Delay` 0.2)
    (`/Game/Blueprints/FrameWorks/GM_BomberAce_GameMode.LevelUpdate` (`self.As GM Bomber Ace Game Mode_0`))
    (`self.K2_DestroyActor`)))

(event `self.DamageArea.OnComponentBeginOverlap`
  (params (OverlappedComponent :type "PrimitiveComponent Object Reference") (OtherActor :type "Actor Object Reference") (OtherComp :type "PrimitiveComponent Object Reference") (OtherBodyIndex :type Integer) (bFromSweep :type Boolean) (SweepResult :type "HitResult Structure (by ref)"))
  (`/Engine/EditorBlueprintResources/StandardMacros.IsValid` OtherActor
    (:`Is Valid`
      (if (`self.ActorHasTag` OtherActor "Player")
        (set `self.Other Actor` OtherActor)
        (set `self.PlaneInRange` true)))))

(event `self.DamageArea.OnComponentEndOverlap`
  (params (OverlappedComponent :type "PrimitiveComponent Object Reference") (OtherActor :type "Actor Object Reference") (OtherComp :type "PrimitiveComponent Object Reference") (OtherBodyIndex :type Integer))
  (`/Engine/EditorBlueprintResources/StandardMacros.IsValid` OtherActor
    (:`Is Valid`
      (if (`self.ActorHasTag` OtherActor "Player")
        (set `self.PlaneInRange` false)))))

(fn `UserConstructionScript`)