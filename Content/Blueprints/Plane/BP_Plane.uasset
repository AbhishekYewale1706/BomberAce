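; Player plane pawn for the Bomber Ace game mode that constantly flies forward, steers by joystick and drops bombs.
; Health and speed load from the "Coin" save slot; Tick turns the joystick vector into a pitch angle via Atan2.
; Bomb fire is gated by a DoOnce that a looping timer resets as a cooldown.
; Lethal damage or enemy overlap explodes and hides the plane, then shows the level-failed widget.
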(event `self.ReceiveBeginPlay`
  (`self.LoadSaveData`)
  (set `self.Health_Div` (`self.Health`))
  (set `FloatingPawnMovement.MaxSpeed` (`self.Speed`) (`self.FloatingPawnMovement`))
  (bind _asgm_bomber_ace_game_mode (cast `/Game/Blueprints/FrameWorks/GM_BomberAce_GameMode` (`GameplayStatics.GetGameMode`)))
  (set `self.As GM Bomber Ace Game Mode` _asgm_bomber_ace_game_mode))

(event `self.ReceiveTick`
  (params (DeltaSeconds :type "Float (single-precision)"))
  (bind (_lastjoystickvector_x _lastjoystickvector_y) (`KismetMathLibrary.BreakVector2D` (`self.LastJoystickVector`)))
  (bind (_returnvalue_x _returnvalue_y) (`KismetMathLibrary.BreakVector2D` (`KismetMathLibrary.Normal2D` (`KismetMathLibrary.MakeVector2D` _lastjoystickvector_x _lastjoystickvector_y))))
  (bind (_returnvalue_roll _returnvalue_pitch) (`KismetMathLibrary.BreakRotator` (`KismetMathLibrary.RInterpTo` (`self.K2_GetActorRotation`) (`KismetMathLibrary.MakeRotator` 0.0 (`KismetMathLibrary.RadiansToDegrees` (`KismetMathLibrary.Atan2` _returnvalue_x _returnvalue_y))) (`GameplayStatics.GetWorldDeltaSeconds`) 250.0)))
  (if (not (`self.IsDead`))
    (`self.AddMovementInput` (`self.GetActorForwardVector`))
    (bind _output_get (set `self.JoystickInput` (`KismetMathLibrary.MakeVector2D` (`self.GetInputAxisValue`) (`self.GetInputAxisValue`))))
    (if (not (> (`KismetMathLibrary.VSize2D` _output_get) 0.1))
      (set `self.LastJoystickVector` (`self.JoystickInput`))
      (else
        (set `self.LastJoystickVector` (`self.JoystickInput`))
        (`self.K2_SetActorRotation` (`KismetMathLibrary.MakeRotator` 0.0 _returnvalue_pitch))))))

(event `self.ReceiveAnyDamage`
  (params (Damage :type "Float (single-precision)") (DamageType :type "DamageType Object Reference") (InstigatedBy :type "Controller Object Reference") (DamageCauser :type "Actor Object Reference"))
  (bind _output_get (set `self.Health` (- (`self.Health`) Damage)))
  (if (<= _output_get 0.0)
    (`self.PlayerDead`)))

(event `self.Box.OnComponentBeginOverlap`
  (params (OverlappedComponent :type "PrimitiveComponent Object Reference") (OtherActor :type "Actor Object Reference") (OtherComp :type "PrimitiveComponent Object Reference") (OtherBodyIndex :type Integer) (bFromSweep :type Boolean) (SweepResult :type "HitResult Structure (by ref)"))
  (`/Engine/EditorBlueprintResources/StandardMacros.IsValid` OtherActor
    (:`Is Valid`
      (if (`ActorComponent.ComponentHasTag` OtherComp "Enemy")
        (set `self.Health` 0.0)
        (`self.PlayerDead`)))))

(event `PlayerDead`
  (bind _returnvalue (`self.K2_GetActorLocation`))
  (`GameplayStatics.SpawnEmitterAtLocation` "/Game/Assets/FX/P_Grenade_Explosion_01.P_Grenade_Explosion_01" _returnvalue)
  (`GameplayStatics.PlaySoundAtLocation` "/Game/Assets/Sounds/GrenadeLauncher_Explosion01.GrenadeLauncher_Explosion01" _returnvalue (struct) 1.0 1.0 0.0 null null null null)
  (`self.DisplayHUD`)
  (`KismetSystemLibrary.Delay` 0.2)
  (`self.DisableInput` (`GameplayStatics.GetPlayerController` 0))
  (set `self.IsDead` true)
  (`self.SetActorHiddenInGame` true)
  (`PrimitiveComponent.SetCollisionEnabled` (`self.Box`) "NoCollision")
  (`PlayerController.SetVirtualJoystickVisibility` (`GameplayStatics.GetPlayerController` 0) false))

(event `DisplayHUD`
  (`KismetSystemLibrary.Delay` 1.0)
  (`AudioComponent.Stop` (`/Game/Blueprints/FrameWorks/GM_BomberAce_GameMode.PlanceBackgroundMusic` (`self.As GM Bomber Ace Game Mode`)))
  (bind _returnvalue (`|CreateWidget` "/Game/Blueprints/HUD/WB_LevelFailed.WB_LevelFailed_C"))
  (bind _output_get (set `self.AsWBGameOverRef` _returnvalue))
  (`UserWidget.AddToViewport` _output_get 0))

(event `StopFire`
  (`KismetSystemLibrary.K2_ClearAndInvalidateTimerHandle` (stale `FireButton` _returnvalue)))

(event `FireButton`
  (bind _missilespawn (`self.MissileSpawn`))
  (`/Engine/EditorBlueprintResources/StandardMacros.DoOnce` false :!label _label
    (:`Completed`
      (`|SpawnActorFromClass` "/Game/Blueprints/Missile/BP_Bomb.BP_Bomb_C" (`KismetMathLibrary.MakeTransform` (`SceneComponent.K2_GetComponentLocation` _missilespawn) (`SceneComponent.K2_GetComponentRotation` _missilespawn)) "Undefined" "MultiplyWithRoot" null null)
      (bind _returnvalue (`KismetSystemLibrary.K2_SetTimerDelegate` (delegate `StartFire`) 0.1 true)))))

(event `Key|SpaceBar`
  (params (Key :type "Key Structure"))
  (:`Pressed`
    (goto _label)))

(event `StartFire`
  (bind _output_get (set `self.FireTime` (- (`self.FireTime`) 0.1)))
  (if (<= _output_get 0.0)
    (`self.StopFire`)
    (set `self.FireTime` 1.0)
    (goto _label :!via `Reset`)))

(event `LoadSaveData`
  (bind _returnvalue (`GameplayStatics.DoesSaveGameExist` "Coin"))
  (if _returnvalue
    (bind _returnvalue_2 (`GameplayStatics.LoadGameFromSlot` "Coin"))
    (bind _asplane_save_game (cast `/Game/Blueprints/SaveGame/PlaneSaveGame` _returnvalue_2))
    (`/Engine/EditorBlueprintResources/StandardMacros.IsValid` _asplane_save_game
      (:`Is Valid`
        (set `self.Health` (`/Game/Blueprints/SaveGame/PlaneSaveGame.Health` _asplane_save_game))
        (set `self.Speed` (`/Game/Blueprints/SaveGame/PlaneSaveGame.Speed` _asplane_save_game))))
    (else
      (bind _returnvalue_3 (`GameplayStatics.CreateSaveGameObject` "/Game/Blueprints/SaveGame/PlaneSaveGame.PlaneSaveGame_C"))
      (`GameplayStatics.SaveGameToSlot` _returnvalue_3 "Coin"))))

(fn `UserConstructionScript`)