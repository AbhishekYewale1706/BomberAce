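; BP_CheckPoint is a level checkpoint pickup that advances the player's progress in the Bomber Ace game mode.
; On BeginPlay it casts and caches GM_BomberAce_GameMode.
; When the player pawn overlaps its sphere, it adds a fixed increment to the game mode's LevelProgressBar and destroys itself.
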(event `self.ReceiveBeginPlay`
  (bind _asgm_bomber_ace_game_mode (cast `/Game/Blueprints/FrameWorks/GM_BomberAce_GameMode` (`GameplayStatics.GetGameMode`)))
  (set `self.As GM Bomber Ace Game Mode` _asgm_bomber_ace_game_mode))

(event `self.Sphere1.OnComponentBeginOverlap`
  (params (OverlappedComponent :type "PrimitiveComponent Object Reference") (OtherActor :type "Actor Object Reference") (OtherComp :type "PrimitiveComponent Object Reference") (OtherBodyIndex :type Integer) (bFromSweep :type Boolean) (SweepResult :type "HitResult Structure (by ref)"))
  (bind _as_gm_bomber_ace_game_mode (`self.As GM Bomber Ace Game Mode`))
  (if (== OtherActor (`GameplayStatics.GetPlayerPawn` 0))
    (set `/Game/Blueprints/FrameWorks/GM_BomberAce_GameMode.level progress bar` (+ (`/Game/Blueprints/FrameWorks/GM_BomberAce_GameMode.level progress bar` _as_gm_bomber_ace_game_mode) 0.15) _as_gm_bomber_ace_game_mode)
    (`self.K2_DestroyActor`)))

(fn `UserConstructionScript`)